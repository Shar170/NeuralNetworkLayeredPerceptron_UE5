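; Neural-network car agent that steers a Character toward the actor tagged "finish", built for generational evolution.
; Each tick, a fan of line-trace hit times plus normalized navmesh path length feeds the network, whose strongest output picks the movement direction.
; Generation zero builds a random-depth ReLU network and briefly pretrains it on synthetic samples.
; Later generations load the parent network, randomly applying reweight mutation at a rate that shrinks with game time.
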(event `self.ReceiveBeginPlay`
  (bind _nnparent_data (`self.NNParent Data`))
  (set `CharacterMovementComponent.MaxWalkSpeed` (`self.Speed`) (`self.CharacterMovement`))
  (bind _newnn1 (`self.F_InitNN` _nnparent_data))
  (set `self.NeuralNetwork` _newnn1)
  (if (== (`.AgentGeneration_5_025638BE489F019DAE3C0E82257B01B3` (break `/Game/NeuralNetwork/Blueprints/St_AgentData` _nnparent_data)) 0)
    (for _ (range 21)
      (`/Engine/EditorBlueprintResources/StandardMacros.FlipFlop`
        (:`A`
          (bind _exampleinput (`self.PretrainData` 1.0))
          (`KismetArrayLibrary.Array_Set` _exampleinput 2)
          (`NeuralNetwork.Train` (`self.NeuralNetwork`) _exampleinput (`|MakeArray` 1.0 0.0 0.0 :!type "Float (single-precision)") 0.1))
        (:`B`
          (bind _exampleinput_2 (`self.PretrainData` 1.0))
          (`KismetArrayLibrary.Array_Set` _exampleinput_2)
          (`NeuralNetwork.Train` (`self.NeuralNetwork`) _exampleinput_2 (`|MakeArray` 0.0 0.0 1.0 :!type "Float (single-precision)") 0.1))))))

(event `self.ReceiveTick`
  (params (DeltaSeconds :type "Float (single-precision)"))
  (`self.Find Path`)
  (set `self.Direction` (0.0 0.0 0.0))
  (bind _tracesout (`self.Sensor`))
  (bind _dataout (`self.Preprocess` _tracesout))
  (bind _output_get (set `self.Last Data Out` _dataout))
  (`KismetArrayLibrary.Array_Append` _output_get (`|MakeArray` (/ (`self.DistanseToTarget`) 40000.0)))
  (bind (_outputs _maxindex) (`NeuralNetwork.ComputeOutputs` (`self.NeuralNetwork`) (`self.Last Data Out`)))
  (bind _returnvalue (`self.RotateToSegmentSensor` _maxindex))
  (`self.AddMovementInput` _returnvalue)
  (set `self.Direction` _returnvalue))

(event `Find Path`
  (bind _outactors (`GameplayStatics.GetAllActorsWithTag` "finish"))
  (bind _returnvalue (`NavigationSystemV1.FindPathToLocationSynchronously` (`self.K2_GetActorLocation`) (`self.K2_GetActorLocation` (`|GetArrayItem` _outactors)) null null))
  (set `self.DistanseToTarget` (`NavigationPath.GetPathLength` _returnvalue)))

(fn `F_InitNN`
  (params (NNParentData :type "/Game/NeuralNetwork/Blueprints/St_AgentData Structure (by ref)"))
  (returns (NewNN1 :type "NeuralNetwork Object Reference"))
  (locals (NewNN :type "NeuralNetwork Object Reference"))
  (bind _newnn (`local.NewNN`))
  (bind _newnn_2 (`local.NewNN`))
  (bind _returnvalue (`|GenericCreateObject` "/Script/NeuralNetworkPlugin.NeuralNetwork"))
  (set `local.NewNN` _returnvalue)
  (if (> (`.AgentGeneration_5_025638BE489F019DAE3C0E82257B01B3` (break `/Game/NeuralNetwork/Blueprints/St_AgentData` NNParentData)) 0)
    (`NeuralNetwork.LoadNetwork` _newnn (`.AgentNN_8_27FF84D34D9C944C8E6C6F84A914ABD3` (break `/Game/NeuralNetwork/Blueprints/St_AgentData` NNParentData))) ; Load inherited data
    (if (`KismetMathLibrary.RandomBool`)
      (bind _returnvalue_2 (`NeuralNetwork.MutateNetwork` _newnn "Reweight" (`KismetMathLibrary.MapRangeClamped` (`GameplayStatics.GetTimeSeconds`) 0.0 7200.0 0.05 0.001)))
      (`NeuralNetwork.LoadNetwork` _newnn _returnvalue_2) ; Load mutated data
    )
    (return (`local.NewNN`))
    (else
      (bind _output_get (set `NeuralNetwork.NumberOfInputs` (+ (`self.SensorsNum`) 1) _newnn_2)) ; Input data channels to NN
      (bind _output_get_2 (set `NeuralNetwork.NumberOfOutputs` 3 _newnn_2)) ; Output
      (bind _neurons_per_layer (`self.GenerateRandomNNArray`)) ; Generates how many neurons there will be in each hidden layer
      (bind _output_get_3 (set `NeuralNetwork.NeuronsPerLayer` _neurons_per_layer _newnn_2))
      (`KismetArrayLibrary.Array_Insert` _output_get_3 _output_get) ; Add input neurons as first layer
      (`KismetArrayLibrary.Array_Add` _output_get_3 _output_get_2) ; Add output neurns as last layer
      (`NeuralNetwork.InitializeNetwork` _newnn_2 :!pinned true) ; Important! After setting the AI settings, initialization must be performed.
      (bind _layers (`self.GetActivationLayers` false "ReLU" (- (`KismetArrayLibrary.Array_Length` (`NeuralNetwork.NeuronsPerLayer` (`local.NewNN`))) 1)))
      (set `NeuralNetwork.ActivationFunctions` _layers (`local.NewNN`))
      (return _newnn_2))))

(fn `GenerateRandomNNArray`
  (returns (`Neurons Per Layer` :type "Array of Integer"))
  (locals (NewLocalVar :type "Array of Integer") (Size :type Integer))
  (`KismetArrayLibrary.Array_Clear` (`local.NewLocalVar`))
  (bind _output_get (set `local.Size` (`KismetMathLibrary.RandomIntegerInRange` 2 15)))
  (for _ (range 1 (+ _output_get 1))
    (`KismetArrayLibrary.Array_Add` (`local.NewLocalVar`) (`KismetMathLibrary.RandomIntegerInRange` 2 30)))
  (return (`local.NewLocalVar`)))

(fn `GetActivationLayers`
  (params (IsRandom :type Boolean) (AllSet :type "ENeuroActivationFunction Enum" :default "Sigmoid") (Size :type Integer))
  (returns (Layers :type "Array of ENeuroActivationFunction Enum"))
  (locals (NewLocalVar_1 :type "Array of ENeuroActivationFunction Enum"))
  (bind _newlocalvar_1 (`local.NewLocalVar_1`))
  (`KismetArrayLibrary.Array_Clear` _newlocalvar_1)
  (for _ (range 1 (+ Size 1))
    (`KismetArrayLibrary.Array_Add` _newlocalvar_1 (select `bool` IsRandom :`false` AllSet :`true` (`KismetArrayLibrary.Array_Random` (`|MakeArray` "Sigmoid" "ReLU" "Tanh" :!type "ENeuroActivationFunction Enum")))))
  (return _newlocalvar_1))

(fn `Preprocess`
  (params (traces :type "Array of HitResult Structure"))
  (returns (DataOut :type "Array of Float (double-precision)"))
  (locals (Data :type "Array of Float (double-precision)"))
  (for _array_element traces
    (`KismetArrayLibrary.Array_Add` (`local.Data`) (`.Time` (`GameplayStatics.BreakHitResult` _array_element))))
  (return (`local.Data`)))

(fn `PretrainData`
  (params (NewItem :type "Float (double-precision)"))
  (returns (ExampleInput :type "Array of Float (double-precision)"))
  (locals (NewLocalVar_0 :type "Array of Float (double-precision)"))
  (for _ (range 1 (+ (`NeuralNetwork.NumberOfInputs` (`self.NeuralNetwork`)) 1))
    (`KismetArrayLibrary.Array_Add` (`local.NewLocalVar_0`) NewItem))
  (return (`local.NewLocalVar_0`)))

(fn `RotateToSegmentSensor`
  (params (A :type Integer))
  (returns (ReturnValue :type "Vector Structure"))
  (bind _sensorsnum (`self.SensorsNum`))
  (return (`KismetMathLibrary.RotateAngleAxis` (`self.GetActorForwardVector`) (`KismetMathLibrary.Conv_IntToDouble` (* (- A (/ _sensorsnum 2)) (/ (`self.FOV`) _sensorsnum))) (0.0 0.0 1.0))))

(fn `Sensor`
  (returns (TracesOut :type "Array of HitResult Structure"))
  (locals (Traces :type "Array of HitResult Structure"))
  (bind _returnvalue (`self.K2_GetActorLocation`))
  (bind _draw_debug_type (`self.Draw Debug Type`))
  (bind _returnvalue_2 (`GameplayStatics.GetPlayerController` 0))
  (bind _returnvalue_3 (`PlayerController.GetHUD` _returnvalue_2))
  (bind _asnn_hud (cast `/Game/NeuralNetwork/Blueprints/NN_HUD` _returnvalue_3)
    (:`then`
      _)
    (:`CastFailed`
      _))
  (for _index (range (`self.SensorsNum`))
    (bind _outhit (`KismetSystemLibrary.LineTraceSingle` :`Start` _returnvalue :`End` (+ _returnvalue (* (`self.RotateToSegmentSensor` _index) 500.0)) :`TraceChannel` "TraceTypeQuery1" :`DrawDebugType` _draw_debug_type))
    (`KismetArrayLibrary.Array_Add` (`local.Traces`) _outhit)
    (if (`|EnumInequality` _draw_debug_type)
      (`/Engine/EditorBlueprintResources/StandardMacros.IsValid` _asnn_hud
        (:`Is Valid`
          (`KismetArrayLibrary.Array_Add` (`/Game/NeuralNetwork/Blueprints/NN_HUD.Textes` _asnn_hud) (`KismetStringLibrary.Conv_IntToString` _index))
          (bind (_bblockinghit _binitialoverlap _time _distance _location _impactpoint _normal _impactnormal _physmat _hitactor _hitcomponent _hitbonename _bonename _hititem _elementindex _faceindex _tracestart _traceend) (`GameplayStatics.BreakHitResult` _outhit))
          (`KismetArrayLibrary.Array_Add` (`/Game/NeuralNetwork/Blueprints/NN_HUD.Positions` _asnn_hud) (`GameplayStatics.ProjectWorldToScreen` _returnvalue_2 (`KismetMathLibrary.SelectVector` _location _traceend _bblockinghit) true))))))
  (return (`local.Traces`)))

(fn `UserConstructionScript`)

(fn `WhatIsSeen`
  (params (IsSeenAny :type Boolean) (Object :type "Object Object Reference"))
  (returns (ReturnValue :type "Float (double-precision)"))
  (return (`KismetMathLibrary.SelectFloat` (`KismetMathLibrary.SelectFloat` 1.0 (`KismetMathLibrary.SelectFloat` 1.5 0.0 (`.bSuccess` (cast `/Game/NeuralNetwork/Blueprints/Actors/BP_ExampleFood` Object :!pure true))) (`.bSuccess` (cast `Pawn` Object :!pure true))) -1.0 IsSeenAny)))