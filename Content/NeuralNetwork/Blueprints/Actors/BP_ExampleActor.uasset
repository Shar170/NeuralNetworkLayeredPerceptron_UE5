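; Neural-network agent for an evolution simulation that senses, moves, attacks and spends energy each tick, dying when depleted.
; Line-trace sensors, heading and start-relative direction feed MovementNeuralNetwork, whose outputs drive both steering and attack traces that steal energy or apply damage.
; High energy spawns children with mutated networks, while deaths respawn fresh, pretrained random-layer agents near TargetPoints, both under a population cap.
; ActionNeuralNetwork is mutated but never evaluated; body color derives from network weights.
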(event `MakeChild`
  (bind _outactors (`GameplayStatics.GetAllActorsOfClass` "BP_ExampleActor_C"))
  (if (< (`KismetArrayLibrary.Array_Length` _outactors) 20)
    (set `self.ChildEnergy` (- (`self.Energy`) 100.0))
    (set `self.Energy` 100.0)
    (bind _outputpin (`self.MutateNNRegions`))
    (bind _returnvalue (`AIBlueprintHelperLibrary.SpawnAIFromClass` (`GameplayStatics.GetObjectClass` self) null (+ (`self.K2_GetActorLocation`) (0.0 0.0 100.0)) (`KismetMathLibrary.MakeRotator` 0.0 0.0 (`KismetMathLibrary.RandomFloatInRange` -180.0 180.0)) true null))
    (bind _asbp_example_actor (cast `/Game/NeuralNetwork/Blueprints/Actors/BP_ExampleActor` _returnvalue))
    (set `/Game/NeuralNetwork/Blueprints/Actors/BP_ExampleActor.ParentData` _outputpin _asbp_example_actor)
    (set `/Game/NeuralNetwork/Blueprints/Actors/BP_ExampleActor.Energy` (`self.ChildEnergy`) _asbp_example_actor)
    (`self.LaunchCharacter` _asbp_example_actor (0.0 0.0 100.0) false false)))

(event `OnDestroyed_Event` :!signature `self.OnDestroyed`
  (params (DestroyedActor :type "Actor Object Reference"))
  (bind _outactors (`GameplayStatics.GetAllActorsOfClass` "BP_ExampleActor_C"))
  (if (< (`KismetArrayLibrary.Array_Length` _outactors) 20)
    (bind _outactors_2 (`GameplayStatics.GetAllActorsOfClass` "/Script/Engine.TargetPoint"))
    (bind _returnvalue_location (`KismetMathLibrary.BreakTransform` (`self.GetTransform` (`KismetArrayLibrary.Array_Random` _outactors_2))))
    (bind _randomlocation (`NavigationSystemV1.K2_GetRandomLocationInNavigableRadius` _returnvalue_location 750.0 null null))
    (`AIBlueprintHelperLibrary.SpawnAIFromClass` (`GameplayStatics.GetObjectClass` self) null (+ _randomlocation (0.0 0.0 150.0)) (`KismetMathLibrary.MakeRotator` 0.0 0.0 (`KismetMathLibrary.RandomFloatInRange` -180.0 180.0)) true null)))

(event `self.ReceiveBeginPlay`
  (add `self.OnDestroyed` (delegate `OnDestroyed_Event`))
  (`KismetSystemLibrary.Delay` 0.2)
  ; init movement NN
  (bind _newnn1 (`self.F_InitNN` (`|GetArrayItem` (`self.ParentData`))))
  (set `self.MovementNeuralNetwork` _newnn1)
  (bind _newnn1_2 (`self.F_InitNN` (`|GetArrayItem` (`self.ParentData`))))
  (set `self.ActionNeuralNetwork` _newnn1_2)
  (`self.Move`)
  (set `self.StartPosition` (`self.K2_GetActorLocation`))
  (bind _returnvalue (`PrimitiveComponent.CreateDynamicMaterialInstance` (`self.Sphere`) 0 "/Game/NeuralNetwork/Material/M_BaseMaterial.M_BaseMaterial" "None"))
  (bind _returnvalue_2 (`self.GetColotByWeight`))
  (`MaterialInstanceDynamic.SetVectorParameterValue` _returnvalue "Color" _returnvalue_2))

(event `Move`
  (bind (_returnvalue_x _returnvalue_y) (`KismetMathLibrary.BreakVector` (`self.GetActorForwardVector`)))
  (bind (_returnvalue_x_2 _returnvalue_y_2) (`KismetMathLibrary.BreakVector` (`KismetMathLibrary.Normal` (- (`self.K2_GetActorLocation`) (`self.StartPosition`)))))
  (if (> (`self.Energy`) 0.0)
    (if (> (`self.Energy`) 200.0)
      (`self.MakeChild`))
    (`self.MovementNeuralNetwork`
      (:`then`
        (bind _tracesout (`self.Sensor`))
        (bind _dataout (`self.Preprocess` _tracesout))
        (bind _output_get (set `self.Last Data Out` _dataout))
        (`KismetArrayLibrary.Array_Append` _output_get (`|MakeArray` _returnvalue_x_2 _returnvalue_y_2))
        (`KismetArrayLibrary.Array_Append` _output_get (`|MakeArray` _returnvalue_x _returnvalue_y))
        (bind (_outputs _maxindex) (`NeuralNetwork.ComputeOutputs` (`self.MovementNeuralNetwork`) (`self.Last Data Out`)))
        (`self.AddMovementInput` (`self.RotateToSegmentSensor` _maxindex))
        (bind _outputs_2 (`NeuralNetwork.ComputeOutputs` (`self.MovementNeuralNetwork`) (`self.Last Data Out`)))
        (set `self.Attack` (0.0 0.0 0.0))
        (for (_array_element _array_index) _outputs_2
          (set `self.Attack` (+ (`self.Attack`) (* (`self.RotateToSegmentSensor` _array_index) _array_element))))
        (`self.TryAttack` (`self.Attack`))
        (set `self.Energy` (- (`self.Energy`) 0.1))
        (`KismetSystemLibrary.DelayUntilNextTick`)
        (`self.Move`))
      (:`else`))
    (else
      (`self.K2_DestroyActor`) ; Death
    )))

(event `TryAttack`
  (params (End :type "Vector Structure"))
  (bind _returnvalue (`self.K2_GetActorLocation`))
  ; Attack
  (bind _outhit (`KismetSystemLibrary.LineTraceSingle` :`Start` _returnvalue :`End` (+ _returnvalue (* End 250.0)) :`TraceChannel` "TraceTypeQuery1" :`DrawDebugType` "ForOneFrame" :`DrawTime` 0.0))
  (if (`self.CanDamageAlive`)
    (bind (_bblockinghit _binitialoverlap _time _distance _location _impactpoint _normal _impactnormal _physmat _hitactor) (`GameplayStatics.BreakHitResult` _outhit))
    (bind _asbp_example_actor (cast `/Game/NeuralNetwork/Blueprints/Actors/BP_ExampleActor` _hitactor)
      (:`then`
        (bind _returnvalue_2 (/ (`/Game/NeuralNetwork/Blueprints/Actors/BP_ExampleActor.Energy` _asbp_example_actor) 2.0))
        (set `self.Energy` (+ (`self.Energy`) _returnvalue_2))
        (set `/Game/NeuralNetwork/Blueprints/Actors/BP_ExampleActor.Energy` _returnvalue_2 _asbp_example_actor))
      (:`CastFailed`
        (`GameplayStatics.ApplyDamage` _hitactor 10.0 null self "/Script/Engine.DamageType" :!label _label)))
    (else
      (goto _label))))

(fn `F_InitNN`
  (params (NNParentData :type "/Game/NeuralNetwork/Blueprints/St_AgentData Structure (by ref)"))
  (returns (NewNN1 :type "NeuralNetwork Object Reference"))
  (locals (NewNN :type "NeuralNetwork Object Reference"))
  (bind _newnn (`local.NewNN`))
  (bind _returnvalue (`|GenericCreateObject` "/Script/NeuralNetworkPlugin.NeuralNetwork"))
  (set `local.NewNN` _returnvalue)
  (if (> (`.AgentGeneration_5_025638BE489F019DAE3C0E82257B01B3` (break `/Game/NeuralNetwork/Blueprints/St_AgentData` NNParentData)) 0)
    (`NeuralNetwork.LoadNetwork` (`local.NewNN`) (`.AgentNN_8_27FF84D34D9C944C8E6C6F84A914ABD3` (break `/Game/NeuralNetwork/Blueprints/St_AgentData` NNParentData))) ; Load inherited data
    (return (`local.NewNN`))
    (else
      (bind _output_get (set `NeuralNetwork.NumberOfInputs` (+ (* (`self.SensorsNum`) 2) 4) _newnn)) ; Input data channels to NN
      (bind _output_get_2 (set `NeuralNetwork.NumberOfOutputs` (`self.SensorsNum`) _newnn)) ; Output
      (bind _neurons_per_layer (`self.GenerateRandomNNArray`)) ; Generates how many neurons there will be in each layer
      (bind _output_get_3 (set `NeuralNetwork.NeuronsPerLayer` _neurons_per_layer _newnn))
      (`KismetArrayLibrary.Array_Insert` _output_get_3 _output_get)
      (`KismetArrayLibrary.Array_Add` _output_get_3 _output_get_2)
      (`NeuralNetwork.InitializeNetwork` _newnn :!pinned true) ; Important! After setting the AI settings, initialization must be performed.
      (bind (_simulatedinputsnn _simulatedoutputsnn) (`self.GeneratePreTrainData` _newnn))
      (`NeuralNetwork.Train` _newnn _simulatedinputsnn _simulatedoutputsnn 0.9) ; preTraint
      (return (`local.NewNN`)))))

(fn `GeneratePreTrainData`
  (params (`Цель` :type "NeuralNetwork Object Reference"))
  (returns (SimulatedInputsNN :type "Array of Float (double-precision)") (SimulatedOutputsNN :type "Array of Float (double-precision)"))
  (locals (NewLocalVar_0 :type "Array of HitResult Structure") (NewLocalVar_1 :type "Array of Float (double-precision)") (NewLocalVar_2 :type "Array of Float (double-precision)") (NewLocalVar_3 :type Integer))
  (for _ (range 1 (+ (`self.SensorsNum`) 1))
    (`KismetArrayLibrary.Array_Add` (`local.NewLocalVar_0`) (`GameplayStatics.MakeHitResult` false)))
  (bind _dataout (`self.Preprocess` (`local.NewLocalVar_0`)))
  (bind _output_get (set `local.NewLocalVar_1` _dataout))
  (set `local.NewLocalVar_3` (- (`NeuralNetwork.NumberOfInputs` `Цель`) (`KismetArrayLibrary.Array_Length` _output_get)))
  (for _ (range 1 (+ (`local.NewLocalVar_3`) 1))
    (`KismetArrayLibrary.Array_Add` (`local.NewLocalVar_1`)))
  (for _ (range 1 (+ (`NeuralNetwork.NumberOfOutputs` `Цель`) 1))
    (`KismetArrayLibrary.Array_Add` (`local.NewLocalVar_2`)))
  (`|VariableSetRef` (`|GetArrayItem` (`local.NewLocalVar_2`) (/ (`NeuralNetwork.NumberOfOutputs` `Цель`) 2)) 1.0)
  (return (`local.NewLocalVar_1`) (`local.NewLocalVar_2`)))

(fn `GenerateRandomNNArray`
  (returns (`Neurons Per Layer` :type "Array of Integer"))
  (locals (Size :type Integer) (NewLocalVar :type "Array of Integer"))
  (`KismetArrayLibrary.Array_Clear` (`local.NewLocalVar`))
  (bind _output_get (set `local.Size` (`KismetMathLibrary.RandomIntegerInRange` 2 15)))
  (for _ (range 1 (+ _output_get 1))
    (`KismetArrayLibrary.Array_Add` (`local.NewLocalVar`) (`KismetMathLibrary.RandomIntegerInRange` 2 30)))
  (return (`local.NewLocalVar`)))

(fn `GetColotByWeight`
  (returns (ReturnValue :type "LinearColor Structure"))
  (locals (Summ :type "Float (double-precision)"))
  (bind _returnvalue (`NeuralNetwork.GetSerializableData` (`self.MovementNeuralNetwork`)))
  (set `local.Summ` 0.0)
  (bind (_numberoflayers _neuronsperlayer _weights) (break `NeuralNetworkData` _returnvalue))
  (bind _variable (`self.sum` _neuronsperlayer)
    (:`Completed`
      (for _array_element _weights
        (set `local.Summ` (+ _array_element (`local.Summ`))))
      (return (`KismetMathLibrary.HSVToRGB` (* (/ (`local.Summ`) (* _variable 3)) 360.0) 1.0 1.0)))))

(fn `MutateNNRegions`
  (returns (OutputPin :type "Array of /Game/NeuralNetwork/Blueprints/St_AgentData Structure"))
  (locals (NewLocalVar_4 :type "Array of /Game/NeuralNetwork/Blueprints/St_AgentData Structure"))
  (bind (_agentfamily _agentgeneration) (break `/Game/NeuralNetwork/Blueprints/St_AgentData` (`|GetArrayItem` (`self.ParentData`))))
  (bind (_agentfamily_2 _agentgeneration_2) (break `/Game/NeuralNetwork/Blueprints/St_AgentData` (`|GetArrayItem` (`self.ParentData`))))
  (bind _returnvalue (`NeuralNetwork.MutateNetwork` (`self.MovementNeuralNetwork`) "Reweight" 0.05))
  (`KismetArrayLibrary.Array_Add` (`local.NewLocalVar_4`) (make `/Game/NeuralNetwork/Blueprints/St_AgentData` (`KismetMathLibrary.SelectName` (`KismetStringLibrary.Conv_StringToName` (`KismetSystemLibrary.GetObjectName` self)) _agentfamily_2 (== _agentgeneration_2 0)) (+ _agentgeneration_2 1) _returnvalue))
  (bind _returnvalue_2 (`NeuralNetwork.MutateNetwork` (`self.ActionNeuralNetwork`) "Reweight" 0.05))
  (`KismetArrayLibrary.Array_Add` (`local.NewLocalVar_4`) (make `/Game/NeuralNetwork/Blueprints/St_AgentData` (`KismetMathLibrary.SelectName` (`KismetStringLibrary.Conv_StringToName` (`KismetSystemLibrary.GetObjectName` self)) _agentfamily (== _agentgeneration 0)) (+ _agentgeneration 1) _returnvalue_2))
  (return (`local.NewLocalVar_4`)))

(fn `Preprocess`
  (params (traces :type "Array of HitResult Structure"))
  (returns (DataOut :type "Array of Float (double-precision)"))
  (locals (Data :type "Array of Float (double-precision)"))
  (bind _data (`local.Data`))
  (for _array_element traces
    (bind (_bblockinghit _binitialoverlap _time _distance _location _impactpoint _normal _impactnormal _physmat _hitactor) (`GameplayStatics.BreakHitResult` _array_element))
    (`KismetArrayLibrary.Array_Add` _data _time)
    (`KismetArrayLibrary.Array_Add` _data (`self.WhatIsSeen` _bblockinghit _hitactor)))
  (return (`local.Data`)))

(fn `RotateToSegmentSensor`
  (params (A :type Integer))
  (returns (ReturnValue :type "Vector Structure"))
  (bind _fov (`self.FOV`))
  (return (`KismetMathLibrary.RotateAngleAxis` (`self.GetActorForwardVector`) (`KismetMathLibrary.Conv_IntToDouble` (- (/ _fov 2) (* A (/ _fov (`self.SensorsNum`))))) (0.0 0.0 1.0))))

(fn `Sensor`
  (returns (TracesOut :type "Array of HitResult Structure"))
  (locals (Traces :type "Array of HitResult Structure"))
  (bind _returnvalue (`self.K2_GetActorLocation`))
  (for _index (range (`self.SensorsNum`))
    (bind _outhit (`KismetSystemLibrary.LineTraceSingle` :`Start` _returnvalue :`End` (+ _returnvalue (* (`self.RotateToSegmentSensor` _index) 500.0)) :`TraceChannel` "TraceTypeQuery1" :`DrawDebugType` (`self.Draw Debug Type`)))
    (`KismetArrayLibrary.Array_Add` (`local.Traces`) _outhit))
  (return (`local.Traces`)))

(fn `UserConstructionScript`)

(fn `WhatIsSeen`
  (params (IsSeenAny :type Boolean) (Object :type "Object Object Reference"))
  (returns (ReturnValue :type "Float (double-precision)"))
  (return (`KismetMathLibrary.SelectFloat` (`KismetMathLibrary.SelectFloat` 1.0 (`KismetMathLibrary.SelectFloat` 1.5 0.0 (`.bSuccess` (cast `/Game/NeuralNetwork/Blueprints/Actors/BP_ExampleFood` Object :!pure true))) (`.bSuccess` (cast `Pawn` Object :!pure true))) -1.0 IsSeenAny)))