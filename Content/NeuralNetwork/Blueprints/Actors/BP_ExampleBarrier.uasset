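; BP_ExampleBarrier is a barrier actor that reacts to any actor overlapping it.
; Characters are launched toward a randomly chosen TargetPoint in the level, with an upward boost added to the direction and their existing velocity overridden.
; Any overlapping actor that is not a Character is destroyed.
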(event `self.ReceiveActorBeginOverlap`
  (params (OtherActor :type "Actor Object Reference"))
  (bind _outactors (`GameplayStatics.GetAllActorsOfClass` "/Script/Engine.TargetPoint"))
  (bind _ascharacter (cast `Character` OtherActor)
    (:`then`
      (bind _returnvalue_location (`KismetMathLibrary.BreakTransform` (`self.GetTransform` (`KismetArrayLibrary.Array_Random` _outactors))))
      (`Character.LaunchCharacter` _ascharacter (* (+ (`KismetMathLibrary.Normal` (- _returnvalue_location (`self.K2_GetActorLocation` OtherActor))) (0.0 0.0 1.0)) 1000.0) true true))
    (:`CastFailed`
      (`self.K2_DestroyActor` OtherActor))))

(fn `UserConstructionScript`)