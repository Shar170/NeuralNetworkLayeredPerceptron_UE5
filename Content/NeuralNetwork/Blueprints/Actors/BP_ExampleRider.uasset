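; BP_ExampleRider is a neural-network example actor that reproduces only when it is near the front of the pack.
; Its MakeChild override finds the shortest navmesh path between the first "RiderEnd"-tagged actor and any BP_ExampleActor.
; The parent MakeChild runs only if the rider's own path to that goal is under 110% of the best, acting as a fitness filter.
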(event `self.MakeChild`
  (bind _outactors (`GameplayStatics.GetAllActorsWithTag` "RiderEnd"))
  (if (`KismetArrayLibrary.Array_IsNotEmpty` _outactors)
    (bind _outactors_2 (`GameplayStatics.GetAllActorsOfClass` "/Game/NeuralNetwork/Blueprints/Actors/BP_ExampleActor.BP_ExampleActor_C"))
    (set `self.BestResult` 100000000000.0)
    (for _array_element _outactors_2
      (bind _output (`|GetArrayItem` _outactors))
      (bind _returnvalue (`self.PathLenght` _array_element _output))
      (if (< _returnvalue (`self.BestResult`))
        (set `self.BestResult` _returnvalue)))
    (bind _returnvalue_2 (`self.PathLenght` _output self))
    (if (< _returnvalue_2 (* (`self.BestResult`) 1.1))
      (`parent.MakeChild`))))

(fn `PathLenght`
  (params (self2 :type "Actor Object Reference") (self3 :type "Actor Object Reference"))
  (returns (ReturnValue :type "Float (double-precision)"))
  (bind _returnvalue (`NavigationSystemV1.FindPathToLocationSynchronously` (`self.K2_GetActorLocation` self3) (`self.K2_GetActorLocation` self2) null "/Script/AIModule.NavFilter_AIControllerDefault"))
  (return (`NavigationPath.GetPathLength` _returnvalue)))

(fn `UserConstructionScript`
  (`parent.UserConstructionScript`))