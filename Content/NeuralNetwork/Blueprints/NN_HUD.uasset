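; NN_HUD is the HUD for the neural network project, showing a control panel and screen-space text labels.
; On BeginPlay it creates WBP_ControlPanel, adds it to the viewport and stores it in the HUD variable.
; DrawHUD draws each Textes entry at its matching Positions coordinate, calls the parent, then empties both arrays, so each queued label lasts a single draw.
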(event `self.ReceiveBeginPlay`
  (bind _returnvalue (`|CreateWidget` "/Game/NeuralNetwork/Blueprints/Widgets/WBP_ControlPanel.WBP_ControlPanel_C"))
  (`UserWidget.AddToViewport` _returnvalue 0)
  (set `self.HUD` _returnvalue))

(event `self.ReceiveDrawHUD`
  (params (SizeX :type Integer) (SizeY :type Integer))
  (for (_array_element _array_index) (`self.Textes`)
    (bind (_x _y) (`KismetMathLibrary.BreakVector2D` (`|GetArrayItem` (`self.Positions`) _array_index)))
    (`self.DrawText` _array_element (struct :`A` 1) _x _y "/Engine/EngineFonts/Roboto.Roboto"))
  (`parent.ReceiveDrawHUD` SizeX SizeY)
  (`KismetArrayLibrary.Array_Clear` (`self.Textes`))
  (`KismetArrayLibrary.Array_Clear` (`self.Positions`)))

(fn `UserConstructionScript`)